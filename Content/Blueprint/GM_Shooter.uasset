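; Shooter game mode that tracks the player's score and creates the score HUD.
; BeginPlay hides the cursor, sets game-only input and adds the WB_Score widget.
; AddScore increases Score and pushes the new total to that widget.
; A completion check for a target score runs only once in BeginPlay, not in AddScore; on a match it shows WB_Complete with cursor and UI-only input.
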(event EventBeginPlay
  (bind _returnvalue (Game|GetPlayerController 0))
  (bind _returnvalue_2 (Game|GetPlayerController 0))
  (Variables|/Script/Engine.PlayerController|SetbShowMouseCursor _returnvalue_2 false)
  (Input|SetInputModeGameOnly _returnvalue_2 false)
  (bind _returnvalue_3 (UserInterface|CreateWidget "/Game/UI/WB_Score.WB_Score_C"))
  (bind _output_get (Variables|Default|SetWB%20Score _returnvalue_3))
  (UserInterface|Viewport|AddtoViewport _output_get 0)
  (if (== (Variables|Default|GetScore) 20)
    (bind _returnvalue_4 (UserInterface|CreateWidget "/Game/UI/WB_Complete.WB_Complete_C"))
    (UserInterface|Viewport|AddtoViewport _returnvalue_4 0)
    (Variables|/Script/Engine.PlayerController|SetbShowMouseCursor _returnvalue true)
    (Input|SetInputModeUIOnly _returnvalue 0 "DoNotLock" false)))

(fn ConstructionScript)

(fn AddScore
  (params (AmountToAdd :type Integer))
  (Variables|Default|SetScore (+ (Variables|Default|GetScore) AmountToAdd))
  (Default|UpdateScore (Variables|Default|GetWB%20Score) (Variables|Default|GetScore)))