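; Enemy AI that patrols random reachable points and, when PawnSensing spots BP_Character, chases, faces and shoots it.
; Shooting plays a montage and line-traces from the weapon barrel, throttled by DoOnce and delay, using Weapon data for mesh, range, damage and fire rate.
; Damage updates a camera-facing health bar widget.
; Death turns on mesh physics, drops BP_Ammunition and hides the bar.
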(event OnSeePawn(PawnSensing)
  (params (Pawn :type Pawn%20Object%20Reference))
  (bind _asbp_character (Utilities|Casting|CastToBP_Character Pawn))
  (Variables|Default|SetIsChasing true)
  (CallFunction|ChasingPlayer _asbp_character))

(event Custom|ChasingPlayer
  (params (Player :type BP%20Character%20Object%20Reference))
  (if (not (Variables|Default|GetIsDeath))
    (AI|AIMoveTo self "0, 0, 0" Player 15.0 false
      (:then
        _)
      (:OnSuccess
        (Variables|Default|SetIsChasing false :!label _label))
      (:OnFail
        (goto _label)))
    (Transformation|SetActorRotation (Math|Rotator|FindLookatRotation (Transformation|GetActorLocation) (Transformation|GetActorLocation Player)))
    (CallFunction|Shoot)))

(event Custom|Patrol
  (if (not (Variables|Default|GetIsDeath))
    (Utilities|FlowControl|Delay 2.0)
    (AI|AIMoveTo self (.RandomLocation (AI|Navigation|GetRandomReachablePointinRadius (Transformation|GetActorLocation) 5e+02 0 0)) 0 5.0 false
      (:OnSuccess
        _)
      (:OnFail
        _))
    (Variables|Default|SetIsChasing (not (Variables|Default|GetIsChasing)))
    (CallFunction|Patrol)))

(event Custom|Shoot
  (bind _armedweapon (Variables|Default|GetArmedWeapon))
  (bind _returnvalue (Transformation|GetSocketLocation _armedweapon "barrel"))
  (Utilities|FlowControl|Sequence
    (:then_0
      (Utilities|FlowControl|DoOnce false :!label _label
        (:Completed
          (Animation|Montage|PlayMontage (Variables|Character|GetMesh) "/Game/Characters/QuantumCharacter/Demo/Animations/AM_Shoot.AM_Shoot" 0.5
            (:then
              (Audio|PlaySoundatLocation "/Game/Audio/404560__superphat__assaultrifle3.404560__superphat__assaultrifle3" _returnvalue "0, 0, 0" 1.0 1.0 0.0 0 0 0 0)
              (bind _outhit (Collision|LineTraceByChannel _returnvalue (+ _returnvalue (* (Math|Vector|GetForwardVector (Transformation|GetActorRotation)) (Variables|/Game/Weapon/Data/BP_WeaponData.BP_WeaponData_C|GetFireDistance (Variables|Default|GetWeapon)))) "TraceTypeQuery1" false 0 "ForDuration" true "(R=1.000000,G=0.000000,B=0.000000,A=1.000000)" "(R=0.000000,G=1.000000,B=0.000000,A=1.000000)" 2.0))
              (bind _asbp_character (Utilities|Casting|CastToBP_Character (.hitactor _outhit)))
              (Game|Damage|ApplyDamage _asbp_character (Variables|/Game/Weapon/Data/BP_WeaponData.BP_WeaponData_C|GetDamage (Variables|Default|GetWeapon)) 0 0))))))
    (:then_1
      (Utilities|FlowControl|Delay (Variables|/Game/Weapon/Data/BP_WeaponData.BP_WeaponData_C|GetFireRate (Variables|Default|GetWeapon)))
      (goto _label Reset))))

(event Game|Damage|EventAnyDamage
  (params (Damage :type Float%20%28single-precision%29) (DamageType :type Damage%20Type%20Object%20Reference) (InstigatedBy :type Controller%20Object%20Reference) (DamageCauser :type Actor%20Object%20Reference))
  (if (not (Variables|Default|GetIsDeath))
    (bind _output_get (Variables|Default|SetHealth (- (Variables|Default|GetHealth) Damage)))
    (Default|SetHealthBar (Variables|Default|GetWB%20Health%20Bar) _output_get (Variables|Default|GetMaxHealth))
    (if (<= _output_get 0.0)
      (Variables|Default|SetIsDeath true)
      (Physics|SetSimulatePhysics (Variables|Character|GetMesh) true)
      (Game|SpawnActorfromClass "/Game/Item/BP_Ammunition.BP_Ammunition_C" (Math|Transform|MakeTransform (Transformation|GetActorLocation) "0, 0, 0" "1.000000,1.000000,1.000000") "Undefined" "MultiplyWithRoot" 0 0)
      (Widget|SetVisibility (Variables|Default|GetWB%20Health%20Bar) "Hidden"))))

(event EventTick
  (params (DeltaSeconds :type Float%20%28single-precision%29))
  (bind _widgethealthbar (Variables|Default|GetWidgetHealthBar))
  (Transformation|SetWorldRotation _widgethealthbar (Math|Rotator|FindLookatRotation (Transformation|GetWorldLocation _widgethealthbar) (Transformation|GetActorLocation (Game|GetPlayerCameraManager 0))) false false))

(event EventBeginPlay
  (CallFunction|Patrol)
  (bind _aswb_health_bar (Utilities|Casting|CastToWB_HealthBar (UserInterface|GetWidget (Variables|Default|GetWidgetHealthBar))))
  (bind _output_get (Variables|Default|SetWB%20Health%20Bar _aswb_health_bar))
  (Default|SetHealthBar _output_get (Variables|Default|GetHealth) (Variables|Default|GetMaxHealth)))

(fn ConstructionScript
  (Components|SkeletalMesh|SetSkeletalMeshAsset (Variables|Default|GetArmedWeapon) (Variables|/Game/Weapon/Data/BP_WeaponData.BP_WeaponData_C|GetMesh (Variables|Default|GetWeapon))))