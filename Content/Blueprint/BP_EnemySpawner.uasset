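; Enemy spawner actor that creates BP_Enemy actors at its own location and rotation, either all at once or in timed batches.
; SpawnEnemy loops to spawn the requested count in one go, adjusting positions on collision but always spawning.
; BatchEnemy calls SpawnEnemy, waits the given interval with a Delay, and loops back until the batch count runs out, always firing at least one batch.
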(event Custom|SpawnEnemy
  (params (SpawnEnemyCount :type Integer))
  (bind _output_get (Variables|Default|SetSpawnEnemyCount SpawnEnemyCount))
  (while (> _output_get 0)
    (Game|SpawnActorfromClass "/Game/Blueprint/BP_Enemy.BP_Enemy_C" (Math|Transform|MakeTransform (Transformation|GetActorLocation) (Transformation|GetActorRotation) "1.000000,1.000000,1.000000") "AdjustIfPossibleButAlwaysSpawn" "MultiplyWithRoot" 0 0)
    (Variables|Default|SetSpawnEnemyCount (- (Variables|Default|GetSpawnEnemyCount) 1))))

(event Custom|BatchEnemy
  (params (BatchEnemyCount :type Integer) (SpawnEnemyPerBatch :type Integer) (Interval :type Float%20%28double-precision%29))
  (Variables|Default|SetBatchEnemyCount BatchEnemyCount)
  (CallFunction|SpawnEnemy SpawnEnemyPerBatch :!label _label)
  (Variables|Default|SetBatchEnemyCount (- (Variables|Default|GetBatchEnemyCount) 1))
  (Utilities|FlowControl|Delay Interval)
  (if (> (Variables|Default|GetBatchEnemyCount) 0)
    (goto _label)))

(fn ConstructionScript)